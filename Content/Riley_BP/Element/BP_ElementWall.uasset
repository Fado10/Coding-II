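; BP_ElementWall is an elemental barrier that only a player with a matching element shield can pass safely.
; On BeginPlay it sets its text label from its ElementType, defaulting to Fire Wall.
; When the third-person character overlaps the cube, its ElementSheild is compared to the wall's type.
; A mismatch prints "Dead", waits briefly and quits the game.
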(event OnComponentBeginOverlap(Cube)
  (params (OverlappedComponent :type Primitive%20Component%20Object%20Reference) (OtherActor :type Actor%20Object%20Reference) (OtherComp :type Primitive%20Component%20Object%20Reference) (OtherBodyIndex :type Integer) (bFromSweep :type Boolean) (SweepResult :type Hit%20Result%20Structure%20%28by%20ref%29))
  (bind _asbp_third_person_character (Utilities|Casting|CastToBP_ThirdPersonCharacter OtherActor))
  (if (not (Utilities|Enum|Equal(Enum) (Variables|/Game/ThirdPerson/Blueprints/BP_ThirdPersonCharacter.BP_ThirdPersonCharacter_C|GetElementSheild _asbp_third_person_character) (Variables|Default|GetElementType)))
    (Development|PrintText "Dead")
    (Utilities|FlowControl|Delay 2.0)
    (Game|QuitGame 0 "Quit" false)))

(event EventBeginPlay
  (Development|PrintText (|GenerictoText (Variables|Default|GetElementType)))
  (switch Utilities|FlowControl|Switch|SwitchonElementalType (Variables|Default|GetElementType)
    (:NewEnumerator0
      (Rendering|Components|TextRender|SetText (Variables|Default|GetTextRender) (Utilities|Text|MakeLiteralText "Fire Wall")))
    (:NewEnumerator1
      (Rendering|Components|TextRender|SetText (Variables|Default|GetTextRender) (Utilities|Text|MakeLiteralText "Earth  Wall")))
    (:NewEnumerator2
      (Rendering|Components|TextRender|SetText (Variables|Default|GetTextRender) (Utilities|Text|MakeLiteralText "Water Wall")))
    (:NewEnumerator3
      (Rendering|Components|TextRender|SetText (Variables|Default|GetTextRender) (Utilities|Text|MakeLiteralText "Fire  Wall")))
    (:NewEnumerator4
      (Rendering|Components|TextRender|SetText (Variables|Default|GetTextRender) (Utilities|Text|MakeLiteralText "Air Wall")))))

(fn ConstructionScript)