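; Machine gun weapon Blueprint that can be picked up, used and dropped, with firing currently only a placeholder "Bang!" print.
; PickUp logs the pickup, snaps the gun to the given skeletal mesh's hand_r socket and disables collision on MachineGunBody.
; Drop detaches it in world space and re-enables collision, briefly simulating physics so it falls before physics is switched off after a short delay.
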(event EventBeginPlay)

(event Collision|EventActorBeginOverlap
  (params (OtherActor :type Actor%20Object%20Reference)))

(event EventTick
  (params (DeltaSeconds :type Float%20%28single-precision%29)))

(event EventPickUp
  (params (SkeletalMesh :type Skeletal%20Mesh%20Component%20Object%20Reference))
  ;[0.15 0.15 0.15 0.5] Pick Up
  (Development|PrintText (Utilities|Text|FormatText "{name} is picked up. Attached to {mesh} " (Utilities|String|MakeLiteralString "Machine Gun") SkeletalMesh) true true "(R=0.136189,G=1.000000,B=0.159645,A=1.000000)" 5.0)
  (Transformation|AttachComponentToComponent SkeletalMesh "hand_r" "SnapToTarget" "SnapToTarget" "SnapToTarget" true)
  (Collision|SetCollisionEnabled (Variables|Default|GetMachineGunBody) "NoCollision"))

(event EventPrimary
  (Development|PrintText "Bang!" true true "(R=1.000000,G=0.346178,B=0.000000,A=1.000000)"))

(event EventDrop
  (bind _machinegunbody (Variables|Default|GetMachineGunBody))
  (Transformation|DetachFromActor "KeepWorld" "KeepWorld" "KeepWorld")
  (Physics|SetSimulatePhysics _machinegunbody true)
  (Collision|SetCollisionEnabled _machinegunbody "QueryAndPhysics")
  (Utilities|FlowControl|Delay 1.0)
  (Physics|SetSimulatePhysics (Variables|Default|GetMachineGunBody) false))

(fn ConstructionScript)